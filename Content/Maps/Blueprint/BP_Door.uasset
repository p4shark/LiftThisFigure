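; Interactable door Blueprint that swings open and closed when the player interacts with it.
; The DoorRotation timeline plays or reverses based on the Openness flag, drives the door's relative yaw, and flips the flag when finished.
; AbilityToOpen is exposed through CanBeInterract, and a separate event prints a "Door close" message for when interaction is not possible.
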(event `/Game/Core/BPI_Interract.Interract`
  (params (Interracted :type "Pawn Object Reference"))
  (if (`self.Openness`)
    (bind (_direction _door) (`Timeline|DoorRotation` :!via `Reverse` :!label _label)
      (:`Update`
        (`SceneComponent.K2_SetRelativeRotation` (`self.Door`) (`KismetMathLibrary.MakeRotator` 0.0 0.0 _door) false false))
      (:`Finished`
        (set `self.Openness` (not (`self.Openness`)))))
    (else
      (goto _label))))

(event `/Game/Core/BPI_Interract.OnCantBeInteracted`
  (`KismetSystemLibrary.PrintString` "Door close. Try to find another way"))

(fn `CanBeInterract`
  (returns (CanBeInterract :type Boolean))
  (return (`self.AbilityToOpen`)))

(fn `UserConstructionScript`)
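; Spawner actor that, on BeginPlay with authority, creates one half-scale BP_FigureBase slightly above itself with a random Id from three types.
; CheckDistributionIsNormal counts the figures already in the world with the candidate Id and accepts it if the count is under six.
; A rejected Id loops back to roll again with no retry limit, capping each type across all spawners.
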(event `self.ReceiveBeginPlay`
  (bind (_returnvalue_location _returnvalue_rotation) (`KismetMathLibrary.BreakTransform` (`self.GetTransform`)))
  (`/Engine/EditorBlueprintResources/ActorMacros.Switch Has Authority`
    (:`Authority`
      (bind (_canbeadd _nnewidadd) (`self.CheckDistributionIsNormal` (`KismetMathLibrary.RandomIntegerInRange` 0 2) :!label _label))
      (if _canbeadd
        (`|SpawnActorFromClass` "/Game/Core/CommandMode/BP_FigureBase.BP_FigureBase_C" (`KismetMathLibrary.MakeTransform` (+ _returnvalue_location (0.0 0.0 50.0)) _returnvalue_rotation (0.5 0.5 0.5)) "Undefined" "OverrideRootScale" null _nnewidadd null)
        (else
          (goto _label))))))

(fn `CheckDistributionIsNormal`
  (params (`New id` :type Integer))
  (returns (CanbeAdd :type Boolean) (NnewIdAdd :type Integer))
  (locals (FigureCounter :type Integer))
  (bind _outactors (`GameplayStatics.GetAllActorsOfClass` "/Game/Core/CommandMode/BP_FigureBase.BP_FigureBase_C"))
  (for _array_element _outactors
    (if (== `New id` (`/Game/Core/CommandMode/BP_FigureBase.Id` _array_element))
      (set `local.FigureCounter` (+ (`local.FigureCounter`) 1))))
  (return (< (`local.FigureCounter`) 6) `New id`))

(fn `UserConstructionScript`)
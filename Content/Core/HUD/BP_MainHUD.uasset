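; Main HUD that shows the match's victory figure and required count, player stats, ability readiness, and the end-game screen.
; On BeginPlay it creates the WBP_HUD widget, binds to BP_GameState dispatchers, then seeds the widget with the current victory goal.
; Handler events forward goal, stat and ability reload updates to the widget.
; EndGame adds a result widget with the victory outcome, and OffHUD removes all widgets.
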(event `self.ReceiveBeginPlay`
  (bind _asbp_game_state (cast `/Game/Core/GameFramework/BP_GameState` (`GameplayStatics.GetGameState`)))
  (set `self.GameState` _asbp_game_state)
  (`self.ForcedHandlerStart`)
  (`|ExecutionSequence`
    (:`then_0`
      (`/Game/Core/HUD/WBP_HUD.InitializeHowFigureNeedForVictory` (`self.MainWidget`) (`/Game/Core/GameFramework/BP_GameState.GetHowFigureNeedToWin` (`self.GameState`))))
    (:`then_1`
      (`/Game/Core/HUD/WBP_HUD.InitializeFigureForVictory` (`self.MainWidget`) (`/Game/Core/CommandMode/BPFL_WorkWithFigure.GetParametersFigureById` (`/Game/Core/GameFramework/BP_GameState.GetTypeFigure` (`self.GameState`)))))))

(event `EndGame`
  (params (Victory :type Boolean))
  (bind _returnvalue (`|CreateWidget` "/Game/Core/HUD/WBP_EndGame.WBP_EndGame_C" null Victory))
  (`UserWidget.AddToViewport` _returnvalue 0))

(event `ForcedHandlerStart`
  (`|ExecutionSequence`
    (:`then_0`
      (bind _returnvalue (`|CreateWidget` "/Game/Core/HUD/WBP_HUD.WBP_HUD_C"))
      (bind _output_get (set `self.MainWidget` _returnvalue))
      (`UserWidget.AddToViewport` _output_get 0))
    (:`then_1`
      (add `/Game/Core/GameFramework/BP_GameState.UpdateHowFigureForVictoryGamestate` (`self.GameState`) (`|CreateDelegate` :!event `InitializeHowFigureNeedForVictory`))
      (add `/Game/Core/GameFramework/BP_GameState.InitializeFigureFOrVictoryGamState` (`self.GameState`) (`|CreateDelegate` :!event `InitializeFigureForVictory`))
      (add `/Game/Core/GameFramework/BP_GameState.UpdateClientStatGameState` (`self.GameState`) (`|CreateDelegate` :!event `UpdateInfo`))
      (add `/Game/Core/GameFramework/BP_GameState.PrintInfoAboutRealodAbilityDispather` (`self.GameState`) (`|CreateDelegate` :!event `PrintInfoAboutHookReadiness`)))))

(event `OffHUD`
  (`WidgetLayoutLibrary.RemoveAllWidgets`))

(event `UpdateInfo`
  (`/Game/Core/HUD/WBP_HUD.CorrectStat` (`self.MainWidget`)))

(event `InitializeHowFigureNeedForVictory`
  (params (HowFigure :type Integer))
  (`/Game/Core/HUD/WBP_HUD.InitializeHowFigureNeedForVictory` (`self.MainWidget`) HowFigure))

(event `InitializeFigureForVictory`
  (params (Figure :type "/Game/Core/CommandMode/S_Figure Structure"))
  (`/Game/Core/HUD/WBP_HUD.InitializeFigureForVictory` (`self.MainWidget`) Figure))

(fn `PrintInfoAboutHookReadiness`
  (params (Time :type "Float (double-precision)") (NameAbility :type Name))
  (`/Game/Core/HUD/WBP_HUD.Print Info About Hook Readiness` (`self.MainWidget`) Time NameAbility))

(fn `UserConstructionScript`)
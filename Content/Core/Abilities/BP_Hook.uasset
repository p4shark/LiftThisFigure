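; BP_Hook is a hook projectile that flies forward from its spawn point and pulls whatever it hits back to that point.
; On the server, a hit or exceeding a maximum range stops the projectile and starts the retraction.
; A timeline lerps the hook from its current location toward the start, teleporting any valid hit actor along slightly below it, then destroys the hook when finished.
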(event `self.ReceiveTick`
  (params (DeltaSeconds :type "Float (single-precision)"))
  (`/Engine/EditorBlueprintResources/ActorMacros.Switch Has Authority`
    (:`Authority`
      (if (> (`KismetMathLibrary.VSize` (- (`self.K2_GetActorLocation`) (`self.StartLocation`))) 2000.0)
        (`self.HookMove` null)))))

(event `self.ReceiveBeginPlay`
  (set `self.StartLocation` (`SceneComponent.K2_GetComponentLocation` (`self.Sphere`)))
  (`ProjectileMovementComponent.SetVelocityInLocalSpace` (`self.ProjectileMovement`) (2000.0 0.0 0.0)))

(event `self.ReceiveHit`
  (params (MyComp :type "PrimitiveComponent Object Reference") (Other :type "Actor Object Reference") (OtherComp :type "PrimitiveComponent Object Reference") (bSelfMoved :type Boolean) (HitLocation :type "Vector Structure") (HitNormal :type "Vector Structure") (NormalImpulse :type "Vector Structure") (Hit :type "HitResult Structure (by ref)"))
  (`/Engine/EditorBlueprintResources/ActorMacros.Switch Has Authority`
    (:`Authority`
      (`self.HookMove` Other))))

(event `HookMove`
  (params (Actor :type "Actor Object Reference"))
  (`ProjectileMovementComponent.SetVelocityInLocalSpace` (`self.ProjectileMovement`) (0.0 0.0 0.0))
  (`self.MoveObject` Actor))

(event `MoveObject`
  (params (Actor :type "Actor Object Reference"))
  (bind (_direction _newtrack_0) (`Timeline|Timeline_0`)
    (:`Update`
      (bind _returnvalue (`KismetMathLibrary.VLerp` (`self.K2_GetActorLocation`) (`self.StartLocation`) _newtrack_0))
      (`self.K2_SetActorLocation` _returnvalue false true)
      (`/Engine/EditorBlueprintResources/StandardMacros.IsValid` Actor
        (:`Is Valid`
          (`self.K2_SetActorLocation` Actor (- _returnvalue (0.0 0.0 25.0)) false true))))
    (:`Finished`
      (`self.K2_DestroyActor`))))

(fn `UserConstructionScript`)
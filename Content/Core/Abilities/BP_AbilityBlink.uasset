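; BP_AbilityBlink is a blink ability that instantly moves its owner forward.
; On UseAbility, it adds a fixed-distance offset along the ability actor's own normalized forward vector to that actor's location, then sets the owner's location to the result.
; The move is a swept teleport, so blocking collision can cut it short.
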(event `/Game/Core/Abilities/BPI_Ability.UseAbility`
  (`self.K2_SetActorLocation` (`self.GetOwner`) (+ (`self.K2_GetActorLocation`) (* (`KismetMathLibrary.Normal` (`self.GetActorForwardVector`)) 1000.0)) true true))

(fn `UserConstructionScript`
  (`parent.UserConstructionScript`))
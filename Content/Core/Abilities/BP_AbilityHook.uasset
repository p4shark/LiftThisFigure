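; Hook ability actor that launches a BP_Hook on behalf of its owner when used.
; The UseAbilityes event passes the owner to CreateAbility, which spawns and returns the hook.
; The spawn point sits a short distance from the actor's location, diagonally forward and up relative to its eye view.
; The hook faces the view direction and receives that spawn point as its StartLocation.
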(event `self.UseAbilityes`
  (`self.CreateAbility` (`self.GetOwner`)))

(fn `CreateAbility`
  (params (Actor :type "Actor Object Reference"))
  (returns (ActorForActivated :type "Actor Object Reference"))
  (bind (_outlocation _outrotation) (`self.GetActorEyesViewPoint` Actor))
  (bind _returnvalue (`KismetMathLibrary.GetForwardVector` _outrotation))
  (bind _returnvalue_2 (+ (`self.K2_GetActorLocation` Actor) (* (`KismetMathLibrary.Normal` (+ _returnvalue (`KismetMathLibrary.GetUpVector` _outrotation))) 100.0)))
  (bind _returnvalue_3 (`|SpawnActorFromClass` "/Game/Core/Abilities/BP_Hook.BP_Hook_C" (`KismetMathLibrary.MakeTransform` _returnvalue_2 (`KismetMathLibrary.Conv_VectorToRotator` _returnvalue)) "Undefined" "OverrideRootScale" null _returnvalue_2 null))
  (return _returnvalue_3))

(fn `UserConstructionScript`
  (`parent.UserConstructionScript`))
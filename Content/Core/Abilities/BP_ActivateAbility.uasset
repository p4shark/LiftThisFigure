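; Helper Blueprint that activates an ability for a given Actor as soon as it begins play.
; It looks up the ability class by Id and spawns it 100 units from the Actor, diagonally along view forward plus up, facing the view direction.
; It then sends UseAbility to the spawned ability through a message call, passing the Actor, and prints the owner and ability name.
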(event `self.ReceiveBeginPlay`
  (bind (_id _name _reloadtime _class) (break `/Game/Core/Abilities/S_Ability` (`/Game/Core/Abilities/BPFL_WorkWithAbility.GetAbilityById` (`self.Id`))))
  (bind _actorforactivated (`self.CreateAbility` (`self.Actor`) _class))
  (message `/Game/Core/Intefraces/BPI_Ability.UseAbility` _actorforactivated (`self.Actor`))
  (`KismetSystemLibrary.PrintString` (`KismetTextLibrary.Conv_TextToString` (`|FormatText` "{owner} use {name}" (`self.Actor`) _name))))

(fn `CreateAbility`
  (params (Actor :type "Actor Object Reference") (class :type "Actor Class Reference"))
  (returns (ActorForActivated :type "Actor Object Reference"))
  (bind (_outlocation _outrotation) (`self.GetActorEyesViewPoint` Actor))
  (bind _returnvalue (`KismetMathLibrary.GetForwardVector` _outrotation))
  (bind _returnvalue_2 (`|SpawnActorFromClass` class (`KismetMathLibrary.MakeTransform` (+ (`self.K2_GetActorLocation` Actor) (* (`KismetMathLibrary.Normal` (+ _returnvalue (`KismetMathLibrary.GetUpVector` _outrotation))) 100.0)) (`KismetMathLibrary.Conv_VectorToRotator` _returnvalue)) "Undefined" "OverrideRootScale" null null))
  (return _returnvalue_2))

(fn `UserConstructionScript`)
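; BP_FigureBase is the base actor for an interactable figure that can be collected when its Id matches the game state's current figure type.
; On server BeginPlay it caches BP_GameState and uses its Id to look up and apply name, static mesh and icon.
; Interacting calls AddFigure on the game state and destroys the actor.
; A helper filters an actor array down to figures with a given Id.
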(event `self.ReceiveBeginPlay`
  (`/Engine/EditorBlueprintResources/ActorMacros.Switch Has Authority`
    (:`Authority`
      (bind _asbp_game_state (cast `/Game/Core/GameFramework/BP_GameState` (`GameplayStatics.GetGameState`)))
      (set `self.MainGameState` _asbp_game_state)
      (bind (_name _staticmesh _icon) (`/Game/Core/BPFL_WorkWithFigure.GetParametersFigureById` (`self.Id`)))
      (set `self.Name` _name)
      (`StaticMeshComponent.SetStaticMesh` (`self.Figure`) _staticmesh)
      (set `self.ImageFigure` _icon))))

(event `/Game/Core/Intefraces/BPI_Interract.Interract`
  (params (Interracted :type "Pawn Object Reference"))
  (`/Game/Core/GameFramework/BP_GameState.AddFigure` (`self.MainGameState`))
  (`self.K2_DestroyActor`))

(fn `CanBeInterract`
  (returns (CanBeInterract :type Boolean))
  (return (== (`/Game/Core/GameFramework/BP_GameState.GetTypeFigure` (`self.MainGameState`)) (`self.Id`))))

(fn `CastActorArrayToFigureBaseArray`
  (params (Array :type "Array of Actor Object Reference") (Type :type Integer))
  (returns (NewParam :type "Array of /Game/Core/BP_FigureBase Object Reference"))
  (locals (LocalArrayFigure :type "Array of /Game/Core/BP_FigureBase Object Reference"))
  (for _array_element Array
    (bind _asbp_figure_base (cast `/Game/Core/BP_FigureBase` _array_element))
    (if (== Type (`/Game/Core/BP_FigureBase.Id` _asbp_figure_base))
      (`KismetArrayLibrary.Array_Add` (`local.LocalArrayFigure`) _asbp_figure_base)))
  (return (`local.LocalArrayFigure`)))

(fn `UserConstructionScript`)
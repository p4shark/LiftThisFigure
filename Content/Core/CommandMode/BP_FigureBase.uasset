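; Base actor for a Command Mode figure, a pickup identified by an Id that reports to BP_GameState when interacted with.
; On BeginPlay, only the authority caches the game state and sets the mesh from the figure parameters for that Id.
; Interaction is allowed when the game state's figure type matches the Id, and Interract adds the figure there and destroys the actor.
; A helper filters actor arrays into figures of a given type.
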(event `self.ReceiveBeginPlay`
  (`/Engine/EditorBlueprintResources/ActorMacros.Switch Has Authority`
    (:`Authority`
      (bind _asbp_game_state (cast `/Game/Core/GameFramework/BP_GameState` (`GameplayStatics.GetGameState`)))
      (set `self.MainGameState` _asbp_game_state)
      (`StaticMeshComponent.SetStaticMesh` (`self.Figure`) (`.StaticMesh_11_CDF2596F4839CDA59F9D8F80D41FA54F` (break `/Game/Core/CommandMode/S_Figure` (`/Game/Core/CommandMode/BPFL_WorkWithFigure.GetParametersFigureById` (`self.Id`))))))))

(event `/Game/Core/BPI_Interract.Interract`
  (params (Interracted :type "Pawn Object Reference"))
  (`/Game/Core/GameFramework/BP_GameState.AddFigure` (`self.MainGameState`))
  (`self.K2_DestroyActor`))

(fn `CanBeInterract`
  (returns (CanBeInterract :type Boolean))
  (return (== (`/Game/Core/GameFramework/BP_GameState.GetTypeFigure` (`self.MainGameState`)) (`self.Id`))))

(fn `CastActorArrayToFigureBaseArray`
  (params (Array :type "Array of Actor Object Reference") (Type :type Integer))
  (returns (NewParam :type "Array of /Game/Core/CommandMode/BP_FigureBase Object Reference"))
  (locals (LocalArrayFigure :type "Array of /Game/Core/CommandMode/BP_FigureBase Object Reference"))
  (for _array_element Array
    (bind _asbp_figure_base (cast `/Game/Core/CommandMode/BP_FigureBase` _array_element))
    (if (== Type (`/Game/Core/CommandMode/BP_FigureBase.Id` _asbp_figure_base))
      (`KismetArrayLibrary.Array_Add` (`local.LocalArrayFigure`) _asbp_figure_base)))
  (return (`local.LocalArrayFigure`)))

(fn `UserConstructionScript`)
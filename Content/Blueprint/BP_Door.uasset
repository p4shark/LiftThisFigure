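; BP_Door is an interactable door that swings open and closed when its Interract event fires.
; The DoorRotation timeline plays forward or in reverse based on IsOpened, driving the door's relative yaw, and flips that flag when finished.
; If CanBeOpen is false, it only prints a message to find another way.
; IsOpened has a RepNotify function, which is empty.
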(event `/Game/Blueprint/BPI_Interract.Interract`
  (params (Interracted :type "Pawn Object Reference"))
  (if (`self.CanBeOpen`)
    (if (`self.IsOpened`)
      (bind (_direction _door) (`Timeline|DoorRotation` :!via `Reverse` :!label _label)
        (:`Update`
          (`SceneComponent.K2_SetRelativeRotation` (`self.Door`) (`KismetMathLibrary.MakeRotator` 0.0 0.0 _door) false false))
        (:`Finished`
          (set `self.IsOpened` (not (`self.IsOpened`)))))
      (else
        (goto _label)))
    (else
      (`KismetSystemLibrary.PrintString` "Door close. Try to find another way"))))

(fn `OnRep_IsOpened`)

(fn `UserConstructionScript`)